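; BP_TestInteractableObject is a clickable test object that shows dialogue in a close-up inspect view.
; Clicking its cube while the player state is free blends to the inspect camera, sends the top-down controller to a walk target and types text into a W_Dialogue widget.
; ExitDialogue blends back to the pawn, frees the state and removes the widget.
; Delays matching blend time gate the focus flag against mid-transition exits.
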(event OnClicked(Cube)
  (params (TouchedComponent :type Primitive%20Component%20Object%20Reference) (ButtonPressed :type Key%20Structure :default "None"))
  (bind _playerstatemanager (Variables|Default|GetplayerStateManager))
  (if (and (Variables|/Game/Blueprints/BP_PlayerStateManager.BP_PlayerStateManager_C|GetisFree (Variables|Default|GetplayerStateManager)) (not (Variables|Default|GetisFocusedOnObject)))
    (Input|EnableInput (Game|GetPlayerController 0))
    (Game|Player|SetViewTargetwithBlend (Game|GetPlayerController 0) (Components|GetOwner (Variables|Default|GetInspectCamera)) 2.0 "VTBlend_EaseInOut" 5.0 false)
    (Default|SetState _playerstatemanager (Variables|/Game/Blueprints/BP_PlayerStateManager.BP_PlayerStateManager_C|GetisInteracting _playerstatemanager))
    (CallFunction|MovePlayertoPosition (Transformation|GetWorldLocation (Variables|Default|GetInspectWalkTarget)))
    (bind _returnvalue (UserInterface|CreateWidget "/Game/Widgets/W_Dialogue.W_Dialogue_C" (Game|GetPlayerController 0)))
    (bind _output_get (Variables|Default|SetdialogueWindow _returnvalue))
    (Default|DisplayDialogueText _output_get (Utilities|String|ToString(Text) (Utilities|Text|FormatText (Utilities|Text|MakeLiteralText (Variables|Default|GetdialogueText)) (Utilities|Text|MakeLiteralText " 
"))) 0.02 self)
    (UserInterface|Viewport|AddtoViewport _output_get 0)
    (Utilities|FlowControl|Delay 2.0)
    (Variables|Default|SetisFocusedOnObject true)))

(event EventExitDialogue
  (bind _playerstatemanager (Variables|Default|GetplayerStateManager))
  (if (and (Variables|/Game/Blueprints/BP_PlayerStateManager.BP_PlayerStateManager_C|GetisInteracting (Variables|Default|GetplayerStateManager)) (Variables|Default|GetisFocusedOnObject))
    (Game|Player|SetViewTargetwithBlend (Game|GetPlayerController 0) (Game|Player|GetPlayerPawn 0) 2.0 "VTBlend_EaseInOut" 5.0 false)
    (Default|SetState _playerstatemanager (Variables|/Game/Blueprints/BP_PlayerStateManager.BP_PlayerStateManager_C|GetisFree _playerstatemanager))
    (Widget|RemovefromParent (Variables|Default|GetdialogueWindow))
    (Input|DisableInput (Game|GetPlayerController 0))
    (Utilities|FlowControl|Delay 2.0)
    (Variables|Default|SetisFocusedOnObject false)))

(event EventBeginPlay
  (bind _asbp_player_state_manager (Utilities|Casting|CastToBP_PlayerStateManager (Game|GetPlayerState 0)))
  (Variables|Default|SetplayerStateManager _asbp_player_state_manager))

(fn ConstructionScript)

(fn MovePlayertoPosition
  (params (targetPosition :type Vector))
  (bind _asbp_top_down_controller (Utilities|Casting|CastToBP_TopDownController (Game|GetPlayerController 0)))
  (Default|Moveto _asbp_top_down_controller targetPosition))