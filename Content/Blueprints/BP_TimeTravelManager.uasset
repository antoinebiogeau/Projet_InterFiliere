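; Manager actor that lets the player press E to jump between parallel past and present copies of a level.
; It teleports the pawn by mapping its position between two landmark components, preserving the relative offset.
; On returning to the present, past objects moved beyond a small tolerance since last check copy their transform, offset to present space, onto their index-paired present counterparts.
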(event EventBeginPlay
  (Input|EnableInput (Game|GetPlayerController 0))
  (for _array_element (Variables|Default|GetpastObjects)
    (Utilities|Array|Add (Variables|Default|GetoldPastObjectPos) (Transformation|GetActorLocation _array_element))))

(event Input|KeyboardEvents|E
  (params (Key :type Key%20Structure :default "None"))
  (:Pressed
    (CallFunction|SwitchTimeline)))

(fn ConstructionScript)

(fn SwitchTimeline
  (if (Variables|Default|GetisInPast)
    (CallFunction|SwitchPlayertoPresent)
    (CallFunction|UpdatePresentObjectPosition)
    (Variables|Default|SetisInPast false)
    (else
      (CallFunction|SwitchPlayertoPast)
      (Variables|Default|SetisInPast true))))

(fn GetPastLocation
  (params (presentLocation :type Vector))
  (return (+ (- presentLocation (Transformation|GetWorldLocation (Variables|Default|GetPresentLandmark))) (Transformation|GetWorldLocation (Variables|Default|GetPastLandmark)))))

(fn GetPresentLocation
  (params (pastLocation :type Vector))
  (return (+ (- pastLocation (Transformation|GetWorldLocation (Variables|Default|GetPastLandmark))) (Transformation|GetWorldLocation (Variables|Default|GetPresentLandmark)))))

(fn SwitchPlayertoPresent
  (bind _presentlocation (CallFunction|GetPresentLocation (Transformation|GetActorLocation (Game|Player|GetPlayerPawn 0))))
  (Transformation|SetActorLocation (Game|Player|GetPlayerPawn 0) _presentlocation false false))

(fn SwitchPlayertoPast
  (bind _pastlocation (CallFunction|GetPastLocation (Transformation|GetActorLocation (Game|Player|GetPlayerPawn 0))))
  (Transformation|SetActorLocation (Game|Player|GetPlayerPawn 0) _pastlocation false false))

(fn UpdatePresentObjectPosition
  (for (_array_element _array_index) (Variables|Default|GetpastObjects)
    (Utilities|HasPastObjectMoved (.location (Transformation|GetActorTransform _array_element)) _array_index
      (:true
        (bind _presentlocation (CallFunction|GetPresentLocation (.location (Transformation|GetActorTransform _array_element))))
        (Transformation|SetActorTransform (Utilities|Array|Get(acopy) (Variables|Default|GetpresentObjects) _array_index) (Math|Transform|MakeTransform _presentlocation (.rotation (Transformation|GetActorTransform _array_element)) (.scale (Transformation|GetActorTransform _array_element))))))))