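; Simon-style memory puzzle actor where the player repeats a random color sequence by overlapping four colored platform colliders.
; Overlapping the start collider generates the sequence, which PlaySequence shows by recoloring one light through delayed self-calls.
; Each color overlap appends to the attempt and rechecks it, flashing the start platform green or red and resetting on a mismatch.
; A full match locks the puzzle and blinks that platform indefinitely.
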(event OnComponentBeginOverlap(Collider)
  (params (OverlappedComponent :type Primitive%20Component%20Object%20Reference) (OtherActor :type Actor%20Object%20Reference) (OtherComp :type Primitive%20Component%20Object%20Reference) (OtherBodyIndex :type Integer) (bFromSweep :type Boolean) (SweepResult :type Hit%20Result%20Structure%20%28by%20ref%29))
  (CallFunction|CreateSequence))

(event OnComponentBeginOverlap(RedCollider)
  (params (OverlappedComponent :type Primitive%20Component%20Object%20Reference) (OtherActor :type Actor%20Object%20Reference) (OtherComp :type Primitive%20Component%20Object%20Reference) (OtherBodyIndex :type Integer) (bFromSweep :type Boolean) (SweepResult :type Hit%20Result%20Structure%20%28by%20ref%29))
  (if (not (Variables|Default|GetPuzzleFinished))
    (if (Variables|Default|GetSequenceCreated)
      (Utilities|Array|Add (Variables|Default|GetPlayerTrySequence) 0)
      (Development|PrintText "RED")
      (CallFunction|CheckPlayerSequence))))

(event OnComponentBeginOverlap(GreenCollider)
  (params (OverlappedComponent :type Primitive%20Component%20Object%20Reference) (OtherActor :type Actor%20Object%20Reference) (OtherComp :type Primitive%20Component%20Object%20Reference) (OtherBodyIndex :type Integer) (bFromSweep :type Boolean) (SweepResult :type Hit%20Result%20Structure%20%28by%20ref%29))
  (if (not (Variables|Default|GetPuzzleFinished))
    (if (Variables|Default|GetSequenceCreated)
      (Utilities|Array|Add (Variables|Default|GetPlayerTrySequence) 3)
      (Development|PrintText "GREEN")
      (CallFunction|CheckPlayerSequence))))

(event OnComponentBeginOverlap(BlueCollider)
  (params (OverlappedComponent :type Primitive%20Component%20Object%20Reference) (OtherActor :type Actor%20Object%20Reference) (OtherComp :type Primitive%20Component%20Object%20Reference) (OtherBodyIndex :type Integer) (bFromSweep :type Boolean) (SweepResult :type Hit%20Result%20Structure%20%28by%20ref%29))
  (if (not (Variables|Default|GetPuzzleFinished))
    (if (Variables|Default|GetSequenceCreated)
      (Utilities|Array|Add (Variables|Default|GetPlayerTrySequence) 1)
      (Development|PrintText "BLUE")
      (CallFunction|CheckPlayerSequence))))

(event OnComponentBeginOverlap(YellowCollider)
  (params (OverlappedComponent :type Primitive%20Component%20Object%20Reference) (OtherActor :type Actor%20Object%20Reference) (OtherComp :type Primitive%20Component%20Object%20Reference) (OtherBodyIndex :type Integer) (bFromSweep :type Boolean) (SweepResult :type Hit%20Result%20Structure%20%28by%20ref%29))
  (if (not (Variables|Default|GetPuzzleFinished))
    (if (Variables|Default|GetSequenceCreated)
      (Utilities|Array|Add (Variables|Default|GetPlayerTrySequence) 2)
      (Development|PrintText "YELLOW")
      (CallFunction|CheckPlayerSequence))))

(event Custom|CheckPlayerSequence
  (for _index (range 0 (- (Utilities|Array|Length (Variables|Default|GetPlayerTrySequence)) 1))
    (if (== (Utilities|Array|Get(acopy) (Variables|Default|GetlightSequence) _index) (Utilities|Array|Get(acopy) (Variables|Default|GetPlayerTrySequence) _index))
      (Development|PrintText "Good")
      (Rendering|Material|SetVectorParameterValue (Variables|Default|GetDynMatInst) "Color" "(R=0.208892,G=1.000000,B=0.190000,A=1.000000)" :!class /Script/Engine.MaterialInstanceDynamic)
      (Utilities|FlowControl|Delay 0.5)
      (Rendering|Material|SetVectorParameterValue (Variables|Default|GetDynMatInst) "Color" "(R=1.000000,G=1.000000,B=1.000000,A=1.000000)" :!class /Script/Engine.MaterialInstanceDynamic)
      (if (== (Utilities|Array|Length (Variables|Default|GetPlayerTrySequence)) (Variables|Default|GetSequenceLenght))
        (Variables|Default|SetPuzzleFinished true)
        (CallFunction|PuzzleComplete))
      (else
        (Development|PrintText "Bad")
        (Variables|Default|SetSequenceCreated false)
        (Variables|Default|Setindex 0)
        (Utilities|Array|Clear (Variables|Default|GetPlayerTrySequence))
        (Rendering|Material|SetVectorParameterValue (Variables|Default|GetDynMatInst) "Color" "(R=0.900000,G=0.000000,B=0.000000,A=1.000000)" :!class /Script/Engine.MaterialInstanceDynamic)
        (Utilities|FlowControl|Delay 2.0)
        (Rendering|Material|SetVectorParameterValue (Variables|Default|GetDynMatInst) "Color" "(R=1.000000,G=1.000000,B=1.000000,A=1.000000)" :!class /Script/Engine.MaterialInstanceDynamic)))))

(event Custom|CreateSequence
  (if (not (Variables|Default|GetPuzzleFinished))
    (if (not (Variables|Default|GetSequenceCreated))
      (Utilities|Array|Clear (Variables|Default|GetlightSequence))
      (for _index (range 0 (- (Variables|Default|GetSequenceLenght) 1))
        (Utilities|Array|Add (Variables|Default|GetlightSequence) (Math|Random|RandomIntegerinRange 0 3)))
      (Variables|Default|SetSequenceCreated true)
      (CallFunction|PlaySequence))))

(event Custom|PlaySequence
  (if (< (Variables|Default|Getindex) (Variables|Default|GetSequenceLenght))
    (Rendering|Components|Light|SetIntensity (Variables|Default|GetLight) 5e+03)
    (switch int (Utilities|Array|Get(acopy) (Variables|Default|GetlightSequence) (Variables|Default|Getindex))
      (:0
        (Development|PrintText "Red")
        (Rendering|Components|Light|SetLightColor (Variables|Default|GetLight) "(R=1.000000,G=0.000000,B=0.054792,A=1.000000)" true))
      (:1
        (Development|PrintText "Blue")
        (Rendering|Components|Light|SetLightColor (Variables|Default|GetLight) "(R=0.000000,G=0.002030,B=1.000000,A=1.000000)" true))
      (:2
        (Development|PrintText "Yellow")
        (Rendering|Components|Light|SetLightColor (Variables|Default|GetLight) "(R=1.000000,G=0.758116,B=0.000000,A=1.000000)" true))
      (:3
        (Development|PrintText "Green")
        (Rendering|Components|Light|SetLightColor (Variables|Default|GetLight) "(R=0.226065,G=1.000000,B=0.000000,A=1.000000)" true)))
    (Utilities|FlowControl|Delay 1.0)
    (Math|Integer|IncrementInt (Variables|Default|Getindex)
      (:%20%20
        (Rendering|Components|Light|SetIntensity (Variables|Default|GetLight) 0.0)
        (Utilities|FlowControl|Delay 0.4)
        (CallFunction|PlaySequence)))))

(event Custom|PuzzleComplete
  (Rendering|Material|SetVectorParameterValue (Variables|Default|GetDynMatInst) "Color" "(R=1.000000,G=1.000000,B=1.000000,A=1.000000)" :!class /Script/Engine.MaterialInstanceDynamic)
  (Utilities|FlowControl|Delay 0.2)
  (Rendering|Material|SetVectorParameterValue (Variables|Default|GetDynMatInst) "Color" "(R=0.208892,G=1.000000,B=0.190000,A=1.000000)" :!class /Script/Engine.MaterialInstanceDynamic)
  (Utilities|FlowControl|Delay 0.2)
  (CallFunction|PuzzleComplete))

(event EventBeginPlay)

(event Collision|EventActorBeginOverlap
  (params (OtherActor :type Actor%20Object%20Reference)))

(event EventTick
  (params (DeltaSeconds :type Float%20%28single-precision%29)))

(fn ConstructionScript
  (Utilities|FlowControl|Sequence
    (:then_0
      (bind _returnvalue (Rendering|Material|CreateDynamicMaterialInstance (Variables|Default|GetRedPlatform) 0 "/Game/Materials/Prototyping/Simon/M_SimonColor_Inst.M_SimonColor_Inst" "None" :!class /Script/Engine.PrimitiveComponent))
      (bind _output_get (Variables|Default|SetDynMatInst _returnvalue))
      (Rendering|Material|SetVectorParameterValue _output_get "Color" "(R=1.000000,G=0.016392,B=0.000000,A=1.000000)" :!class /Script/Engine.MaterialInstanceDynamic))
    (:then_1
      (bind _returnvalue_2 (Rendering|Material|CreateDynamicMaterialInstance (Variables|Default|GetBluePlatform) 0 "/Game/Materials/Prototyping/Simon/M_SimonColor_Inst.M_SimonColor_Inst" "None" :!class /Script/Engine.PrimitiveComponent))
      (bind _output_get_2 (Variables|Default|SetDynMatInst _returnvalue_2))
      (Rendering|Material|SetVectorParameterValue _output_get_2 "Color" "(R=0.000000,G=0.067530,B=1.000000,A=1.000000)" :!class /Script/Engine.MaterialInstanceDynamic))
    (:then_2
      (bind _returnvalue_3 (Rendering|Material|CreateDynamicMaterialInstance (Variables|Default|GetYellowPlatform) 0 "/Game/Materials/Prototyping/Simon/M_SimonColor_Inst.M_SimonColor_Inst" "None" :!class /Script/Engine.PrimitiveComponent))
      (bind _output_get_3 (Variables|Default|SetDynMatInst _returnvalue_3))
      (Rendering|Material|SetVectorParameterValue _output_get_3 "Color" "(R=1.000000,G=0.990346,B=0.000000,A=1.000000)" :!class /Script/Engine.MaterialInstanceDynamic))
    (:then_3
      (bind _returnvalue_4 (Rendering|Material|CreateDynamicMaterialInstance (Variables|Default|GetGreenPlatform) 0 "/Game/Materials/Prototyping/Simon/M_SimonColor_Inst.M_SimonColor_Inst" "None" :!class /Script/Engine.PrimitiveComponent))
      (bind _output_get_4 (Variables|Default|SetDynMatInst _returnvalue_4))
      (Rendering|Material|SetVectorParameterValue _output_get_4 "Color" "(R=0.104063,G=1.000000,B=0.000000,A=1.000000)" :!class /Script/Engine.MaterialInstanceDynamic))
    (:then_4
      (bind _returnvalue_5 (Rendering|Material|CreateDynamicMaterialInstance (Variables|Default|GetStartPlatform) 0 "/Game/Materials/Prototyping/Simon/M_SimonColor_Inst.M_SimonColor_Inst" "None" :!class /Script/Engine.PrimitiveComponent))
      (bind _output_get_5 (Variables|Default|SetDynMatInst _returnvalue_5))
      (Rendering|Material|SetVectorParameterValue _output_get_5 "Color" "(R=1.000000,G=1.000000,B=1.000000,A=1.000000)" :!class /Script/Engine.MaterialInstanceDynamic))))